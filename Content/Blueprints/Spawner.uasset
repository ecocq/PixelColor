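; Spawner actor that builds a grid of PixelCube actors centered on itself at BeginPlay and recolors them in patterns.
; Each cube is stored in a flat PixelArray and receives its index and a Spawner reference.
; Events color a line in one of four directions chosen by angle, diagonals, or a sized square around an index.
; Row and column arithmetic on the flat index, with validity and same-row checks, bounds the patterns.
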(event `self.ReceiveBeginPlay`
  ;[1 1 1] Begin play
  (`self.InitSpawn`)
  (while (< (`self.i`) (`self.rows`))
    (set `self.y` (`self.initialY`))
    (set `self.j` 0)
    (while (< (`self.j`) (`self.columns`))
      (`self.spawnAPixel`))
    (set `self.x` (- (`self.x`) (`self.distance`)))
    (`/Engine/EditorBlueprintResources/StandardMacros.IncrementInt` (`self.i`))))

(event `colorLine`
  (params (index :type Integer) (color :type "LinearColor Structure") (angle :type "Float (double-precision)"))
  ;[1 1 1] color Line
  (`KismetSystemLibrary.PrintString` (`KismetStringLibrary.Conv_DoubleToString` angle) true true (struct :`G` 0.66 :`B` 1.0 :`A` 1.0) 10.0)
  (if (`KismetMathLibrary.InRange_FloatFloat` angle -45.0 45.0 true false)
    (`self.colorOrientedLine` index color true)
    (elif (`KismetMathLibrary.InRange_FloatFloat` angle 45.0 135.0 true false)
      (`self.colorOrientedLine` index color false true)
      (elif (`KismetMathLibrary.InRange_FloatFloat` angle -135.0 -45.0 true false)
        (`self.colorOrientedLine` index color)
        (else
          (`self.colorOrientedLine` index color true true))))))

(event `color Diagonals`
  (params (Index :type Integer) (Color :type "LinearColor Structure"))
  (bind _j (`self.j`))
  (bind _j_2 (`self.j`))
  (bind _returnvalue (- (`self.i`) (* (`self.columns`) _j_2)))
  (bind _returnvalue_2 (+ (`self.i`) (* (`self.columns`) _j)))
  (bind _returnvalue_3 (- _returnvalue_2 _j))
  (bind _returnvalue_4 (- _returnvalue _j_2))
  (bind _returnvalue_5 (+ _returnvalue_2 _j))
  (bind _returnvalue_6 (+ _returnvalue _j_2))
  ;[1 1 1] color Doagonals
  (`/Game/Blueprints/PixelCube.changeColor` (`KismetArrayLibrary.Array_Get` (`self.pixelArray`) Index) Color)
  (set `self.i` Index)
  (set `self.j` 1)
  (set `self.counter` 0)
  (while (<= (`self.counter`) 3)
    (set `self.counter` 0)
    (`self.isValidAndSameRow` _returnvalue_4 _returnvalue
      (:`True`
        (`/Game/Blueprints/PixelCube.changeColor` (`KismetArrayLibrary.Array_Get` (`self.pixelArray`) _returnvalue_4) Color))
      (:`False`
        (`/Engine/EditorBlueprintResources/StandardMacros.IncrementInt` (`self.counter`)
          (:`  `
            _))))
    (`self.isValidAndSameRow` _returnvalue_6 _returnvalue
      (:`True`
        (`/Game/Blueprints/PixelCube.changeColor` (`KismetArrayLibrary.Array_Get` (`self.pixelArray`) _returnvalue_6) Color))
      (:`False`
        (`/Engine/EditorBlueprintResources/StandardMacros.IncrementInt` (`self.counter`)
          (:`  `
            _))))
    (`self.isValidAndSameRow` _returnvalue_3 _returnvalue_2
      (:`True`
        (`/Game/Blueprints/PixelCube.changeColor` (`KismetArrayLibrary.Array_Get` (`self.pixelArray`) _returnvalue_3) Color))
      (:`False`
        (`/Engine/EditorBlueprintResources/StandardMacros.IncrementInt` (`self.counter`)
          (:`  `
            _))))
    (`self.isValidAndSameRow` _returnvalue_5 _returnvalue_2
      (:`True`
        (`/Game/Blueprints/PixelCube.changeColor` (`KismetArrayLibrary.Array_Get` (`self.pixelArray`) _returnvalue_5) Color))
      (:`False`
        (`/Engine/EditorBlueprintResources/StandardMacros.IncrementInt` (`self.counter`)
          (:`  `
            _))))
    (`/Engine/EditorBlueprintResources/StandardMacros.IncrementInt` (`self.j`))))

(event `color Square`
  (params (index :type Integer) (color :type "LinearColor Structure") (size :type Integer))
  (bind _j (`self.j`))
  (bind _returnvalue (- (`self.i`) (* (`self.columns`) (`self.counter`))))
  ;[1 1 1] color Square
  (`/Game/Blueprints/PixelCube.changeColor` (`KismetArrayLibrary.Array_Get` (`self.pixelArray`) index) color)
  (set `self.i` index)
  (set `self.counter` size)
  (while (>= (`self.counter`) (* size -1))
    (set `self.j` (- _returnvalue size))
    (while (<= (`self.j`) (+ _returnvalue size))
      (`self.isValidAndSameRow` _j _returnvalue
        (:`True`
          (`/Game/Blueprints/PixelCube.changeColor` (`KismetArrayLibrary.Array_Get` (`self.pixelArray`) _j) color))
        (:`False`
          _))
      (`/Engine/EditorBlueprintResources/StandardMacros.IncrementInt` (`self.j`)))
    (`/Engine/EditorBlueprintResources/StandardMacros.DecrementInt` (`self.counter`))))

(fn `UserConstructionScript`)