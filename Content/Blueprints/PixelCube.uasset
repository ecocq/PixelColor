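; PixelCube is a single colorable cube actor that works as one indexed pixel under a Spawner.
; Its construction script gives the cube a dynamic material instance, whose Color parameter the changeColor event sets.
; Line, diagonal and square coloring events pass the cube's Index to the Spawner, which handles those patterns, with square size fixed at one.
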(event `changeColor`
  (params (newColor :type "LinearColor Structure"))
  ;[1 1 1] change Color
  (`MaterialInstanceDynamic.SetVectorParameterValue` (`self.material`) "Color" newColor))

(event `colorLine`
  (params (`new Color` :type "LinearColor Structure") (angle :type "Float (double-precision)"))
  ;[1 1 1] color Line
  (`/Game/Blueprints/Spawner.colorLine` (`self.spawner`) (`self.index`) `new Color` angle))

(event `color Diagonals`
  (params (Color :type "LinearColor Structure"))
  ;[1 1 1] color Diagonals
  (`/Game/Blueprints/Spawner.color Diagonals` (`self.spawner`) (`self.index`) Color))

(event `color Square`
  (params (color :type "LinearColor Structure"))
  ;[1 1 1] color Square
  (`/Game/Blueprints/Spawner.color Square` (`self.spawner`) (`self.index`) color 1))

(fn `UserConstructionScript`
  (bind _returnvalue (`PrimitiveComponent.CreateDynamicMaterialInstance` (`self.Cube`) 0 "/Game/Materials/PixelCubeMaterial.PixelCubeMaterial"))
  (set `self.material` _returnvalue)
  (`PrimitiveComponent.SetMaterial` (`self.Cube`) 0 _returnvalue))